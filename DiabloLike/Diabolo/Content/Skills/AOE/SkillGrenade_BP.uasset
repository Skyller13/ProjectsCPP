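; Grenade area-of-effect skill: plays the owner's toss montage, launches the grenade and deals damage where it explodes.
; A physics event detaches the referenced grenade, enables simulation and impulses it along the owner's forward vector.
; The explosion event spawns particles and a detection mesh at the grenade's location.
; Overlaps damage living Damageable actors through HealthComponent, using ActorList, cleared each throw, to prevent repeat hits.
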(event EventEventThrowGrenade
  (bind _skillmanagercomponent (Variables|Default|GetSkillManagerComponent))
  (bind _returnvalue (Class|SkillManagerComponent|GetOwnerCharacter _skillmanagercomponent))
  (Utilities|IsValid _returnvalue
    (:Is%20Valid
      (bind _output_get (Variables|Default|SetOwner _returnvalue))
      (Animation|PlayAnimMontage _output_get "/Game/Animations/Weapons/Grenade/Toss_Grenade_Montage.Toss_Grenade_Montage" 1.2 "None")
      (Utilities|Array|Clear (Variables|Default|GetactorList)))))

(event EventEventonExplosionEvent
  (bind _grenaderef (Variables|Default|GetgrenadeRef))
  (bind _returnvalue (Actor|GetComponentbyClass _grenaderef "/Script/Engine.StaticMeshComponent"))
  (bind _returnvalue_2 (Transformation|GetWorldLocation _returnvalue))
  (Utilities|IsValid _grenaderef
    (:Is%20Valid
      (Effects|SpawnEmitterAttached "/Game/FXVarietyPack/Particles/P_ky_explosion.P_ky_explosion" _returnvalue "None" _returnvalue_2 "0, 0, 0" "1.500000,1.500000,1.500000" "KeepWorldPosition")
      (Class|SkillAttack|SpawnDetectionMeshSpecificTransform (Math|Transform|MakeTransform _returnvalue_2 "0, 0, 0" "1.500000,1.500000,1.500000")))))

(event EventEventSetGrenadePhysics
  (bind _grenaderef (Variables|Default|GetgrenadeRef))
  (bind _returnvalue (Actor|GetComponentbyClass _grenaderef "/Script/Engine.StaticMeshComponent"))
  (Variables|Default|SetisGrenadeThrew true)
  (Transformation|DetachFromActor _grenaderef "KeepWorld" "KeepWorld" "KeepWorld")
  (if (Physics|IsSimulatingPhysics _returnvalue "None")
    _
    (else
      (Physics|SetSimulatePhysics _returnvalue true)))
  (Collision|SetCollisionResponsetoAllChannels _returnvalue "ECR_Block")
  (Collision|SetCollisionResponsetoChannel _returnvalue "ECC_Pawn" "ECR_Overlap")
  (Collision|SetCollisionEnabled _returnvalue "PhysicsOnly")
  (bind _output_get (Variables|Default|SetImpulseDirection (Transformation|GetActorForwardVector (Variables|Default|GetOwner))))
  (Physics|AddImpulse _returnvalue (* _output_get 5e+03) "None" true))

(event EventEventSkillBeginOverlap
  (params (OverlappedComponent :type Primitive%20Component%20Object%20Reference) (OtherActor :type Actor%20Object%20Reference) (OtherComp :type Primitive%20Component%20Object%20Reference) (OtherBodyIndex :type Integer) (bFromSweep :type Boolean) (SweepResult :type Hit%20Result%20Structure%20%28by%20ref%29))
  (bind _returnvalue (Actor|GetComponentbyClass OtherActor "/Script/Diabolo.HealthComponent"))
  (if (and (Utilities|DoesObjectImplementInterface OtherActor "/Script/Diabolo.Damageable") (not (Utilities|Array|ContainsItem (Variables|Default|GetactorList) OtherActor)))
    (Utilities|IsValid _returnvalue
      (:Is%20Valid
        (if (Class|HealthComponent|IsOwnerAlive _returnvalue)
          (Utilities|Array|AddUnique (Variables|Default|GetactorList) OtherActor)
          (Effects|SpawnEmitterAttached "/Game/Particles/FX_Fire_Hit.FX_Fire_Hit" (Variables|/Script/Engine.Actor|GetRootComponent OtherActor) "None" (Transformation|GetActorLocation OtherActor) "0, 0, 0" "1.000000,1.000000,1.000000" "KeepWorldPosition")
          (Class|HealthComponent|RemoveHealth _returnvalue (Math|Conversions|ToFloat(Integer) (Variables|Default|Getdamage))))))))
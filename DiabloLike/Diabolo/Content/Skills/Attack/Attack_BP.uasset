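; Attack skill Blueprint that plays a sped-up attack montage on the owning character and damages what it hits.
; On execute it caches the owner from the skill manager component.
; On skill overlap it filters for living Damageable actors of a different class than the owner, recording each in a list to prevent repeat hits.
; Each valid target gets a fire hit particle and loses health through its HealthComponent.
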(event EventEventExecute
  (bind _skillmanagercomponent (Variables|Default|GetSkillManagerComponent))
  (bind _returnvalue (Class|SkillManagerComponent|GetOwnerCharacter _skillmanagercomponent))
  (Utilities|IsValid _returnvalue
    (:Is%20Valid
      (bind _output_get (Variables|Default|SetOwner _returnvalue))
      (Animation|PlayAnimMontage _output_get (Variables|Default|GetAnimMontage) 1.35 "None"))))

(event EventEventSkillBeginOverlap
  (params (OverlappedComponent :type Primitive%20Component%20Object%20Reference) (OtherActor :type Actor%20Object%20Reference) (OtherComp :type Primitive%20Component%20Object%20Reference) (OtherBodyIndex :type Integer) (bFromSweep :type Boolean) (SweepResult :type Hit%20Result%20Structure%20%28by%20ref%29))
  (bind _returnvalue (Actor|GetComponentbyClass OtherActor "/Script/Diabolo.HealthComponent"))
  (if (Math|Boolean|ANDBoolean (Utilities|DoesObjectImplementInterface OtherActor "/Script/Diabolo.Damageable") (!= (Utilities|GetClass OtherActor) (Utilities|GetClass (Variables|Default|GetOwner))) (not (Utilities|Array|ContainsItem (Variables|Default|GetactorList) OtherActor)))
    (Utilities|IsValid _returnvalue
      (:Is%20Valid
        (if (Class|HealthComponent|IsOwnerAlive _returnvalue)
          (Utilities|Array|AddUnique (Variables|Default|GetactorList) OtherActor)
          (Effects|SpawnEmitterAttached "/Game/Particles/FX_Fire_Hit.FX_Fire_Hit" (Variables|/Script/Engine.Actor|GetRootComponent OtherActor) "None" (Transformation|GetActorLocation OtherActor) "0, 0, 0" "1.000000,1.000000,1.000000" "KeepWorldPosition")
          (Class|HealthComponent|RemoveHealth _returnvalue (Math|Conversions|ToFloat(Integer) (Variables|Default|Getdamage))))))))
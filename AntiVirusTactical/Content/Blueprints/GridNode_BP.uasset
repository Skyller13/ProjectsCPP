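; GridNode_BP is a grid node Blueprint that shows visual feedback for its selection and reset state.
; On BeginPlay it binds handlers to the node's selected, unselected and reset events.
; Selection and unselection toggle the PlaneSelection component's visibility, while reset hides the PlaneRange component.
; This graph only ever hides PlaneRange, and the construction script is empty.
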(event Custom|OnNodeSelect
  (Rendering|SetVisibility (Variables|Default|GetPlaneSelection) true false))

(event Custom|OnNodeUnselect
  (Rendering|SetVisibility (Variables|Default|GetPlaneSelection) false false))

(event Custom|OnNodeReset_Event
  (Rendering|SetVisibility (Variables|Default|GetPlaneRange) false false))

(event EventBeginPlay
  (EventDispatchers|BindEventtoOnNodeSelected (delegate Custom|OnNodeSelect))
  (EventDispatchers|BindEventtoOnNodeUnselected (delegate Custom|OnNodeUnselect))
  (EventDispatchers|BindEventtoOnNodeReset (delegate Custom|OnNodeReset_Event)))

(fn ConstructionScript)
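; Controller logic for grid-based tactical play in AntiVirus, handling node selection and character switching.
; Selection resolves a location through the gamemode's grid and moves the highlight; Attack mode accepts only non-obstacle nodes holding a VirusCharacter within range.
; Switching blends the camera to the new character, then possesses it and begins its turn.
; A helper returns the synchronous navigation path length to a free node.
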(event EventOnPossessSwitchCameraEvent
  (params (_newPlayer :type Anti%20Virus%20Tactical%20Character%20Object%20Reference))
  (bind _returnvalue (Game|GetPlayerController 0))
  ;[1 1 1] Switch characters (With camera blend)
  (Game|Player|SetViewTargetwithBlend _returnvalue _newPlayer 1.0 "VTBlend_Linear" 0.0 false)
  (Utilities|FlowControl|Delay 1.0)
  (Pawn|Possess _returnvalue _newPlayer)
  (Default|CallOnBeginTurnEvent _newPlayer))

(event EventChangeNodeSelectionEvent
  (params (NodeLocation :type Vector :default "0, 0, 0"))
  (bind _returnvalue (Game|GetPlayerController 0))
  (bind _returnvalue_2 (Pawn|GetControlledPawn _returnvalue))
  (bind _asanti_virus_tactical_character (Utilities|Casting|CastToAntiVirusTacticalCharacter _returnvalue_2))
  (bind _asanti_virus_gamemode (Utilities|Casting|CastToAntiVirusGamemode (Game|GetGameMode)))
  (Utilities|IsValid _asanti_virus_gamemode
    (:Is%20Valid
      (bind _asgrid_bp (Utilities|Casting|CastTogrid_BP (Class|AntiVirusTacticalGameMode|GetGrid _asanti_virus_gamemode)))
      (bind (_isvalid _row _column) (Default|LocationtoTile _asgrid_bp NodeLocation))
      (if _isvalid
        (bind _node (Default|GetLinearIndex _asgrid_bp _row _column))
        (Utilities|IsValid _node
          (:Is%20Valid
            (bind _asanti_virus_tactical_player_controller (Utilities|Casting|CastToAntiVirusTacticalPlayerController _returnvalue))
            (switch Utilities|FlowControl|Switch|SwitchonECurrentAction (Variables|/Script/AntiVirusTactical.AntiVirusTacticalPlayerController|GetCurrentAction _asanti_virus_tactical_player_controller)
              (:Walk
                (if (Utilities|IsValid (Variables|Default|GetcurrentSelection))
                  (bind _asgrid_node_bp (Utilities|Casting|CastToGridNode_BP (Variables|Default|GetcurrentSelection) :!label _label))
                  (Default|OnNodeUnselect _asgrid_node_bp))
                (bind _output_get (Variables|Default|SetcurrentSelection _node :!label _label_2))
                (bind _asgrid_node_bp_2 (Utilities|Casting|CastToGridNode_BP _output_get))
                (Default|OnNodeSelect _asgrid_node_bp_2))
              (:Attack
                (Utilities|IsValid (Variables|/Script/AntiVirusTactical.GridNode|GetLinkedActor _node)
                  (:Is%20Valid
                    (Utilities|Casting|CastToVirusCharacter (Variables|/Script/AntiVirusTactical.GridNode|GetLinkedActor _node))
                    (if (Math|Boolean|ANDBoolean (not (Variables|/Script/AntiVirusTactical.GridNode|GetisObstacle _node)) (Utilities|IsValid _asanti_virus_tactical_character) (<= (* (Math|Float|Floor (* (Math|Vector|Distance(Vector) (Transformation|GetActorLocation _node) (Transformation|GetActorLocation (Variables|/Script/AntiVirusTactical.AntiVirusTacticalCharacter|GetplayerNode _asanti_virus_tactical_character))) 0.01)) 1e+02) (* (Variables|/Script/AntiVirusTactical.AntiVirusTacticalCharacter|GetrangeAttack _asanti_virus_tactical_character) 1e+02)))
                      (if (Utilities|IsValid (Variables|Default|GetcurrentSelection))
                        (goto _label)
                        (else
                          (goto _label_2))))))))))))))

(fn ConstructionScript)

(fn GetPathtoNodeEvent
  (params (_startNode :type Grid%20Node%20Object%20Reference) (_hitLocation :type Vector :default "0, 0, 0"))
  (bind _returnvalue (Transformation|GetActorLocation _startNode))
  (bind _asanti_virus_gamemode (Utilities|Casting|CastToAntiVirusGamemode (Game|GetGameMode)))
  (bind _asgrid_bp (Utilities|Casting|CastTogrid_BP (Class|AntiVirusTacticalGameMode|GetGrid _asanti_virus_gamemode)))
  (bind (_isvalid _row _column) (Default|LocationtoTile _asgrid_bp _hitLocation))
  (if _isvalid
    (bind _node (Default|GetLinearIndex _asgrid_bp _row _column))
    (Utilities|IsValid _node
      (:Is%20Valid
        (if (and (== (Variables|/Script/AntiVirusTactical.GridNode|GetLinkedActor _node) 0) (not (Variables|/Script/AntiVirusTactical.GridNode|GetisObstacle _node)))
          (bind _returnvalue_2 (Class|NavigationSystemV1|FindPathtoLocationSynchronously (Math|Vector|MakeVector (.x _returnvalue) (.y _returnvalue) 0.0) (Math|Vector|MakeVector (.x (Transformation|GetActorLocation _node)) (.y (Transformation|GetActorLocation _node)) 0.0) 0 0))
          (return (Class|NavigationPath|GetPathLength _returnvalue_2)))))))
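; Grid-based virus enemy for the AntiVirus tactical game that moves, attacks player characters and can replicate itself.
; BeginPlay claims a random free node, registers in the GameMode's Enemies and initializes its life widget.
; CheckEnemyNearby scans MoveRange, targets by shortest nav path and flags adjacency; Attack plays a montage and damages that target.
; RandomMovement and SpawnVirus use free offset nodes; IsForcingSpawn makes copies skip random placement, and they start with HasPlayed set.
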(event EventBeginPlay
  (bind _self self)
  (bind _self_2 self)
  (if (not (Variables|Default|GetisForcingSpawn))
    (bind _returnvalue (Actor|GetActorOfClass "/Game/Blueprints/grid_BP.grid_BP_C"))
    (bind _output_get (Variables|Default|SetGrid _returnvalue))
    (bind _output_get_2 (Variables|Default|SetLinkedNode (Utilities|Array|Get(acopy) (Variables|/Game/Blueprints/grid_BP.grid_BP_C|GetNodesList _output_get) (Math|Random|RandomIntegerinRange 0 (Utilities|Array|Length (Variables|/Game/Blueprints/grid_BP.grid_BP_C|GetNodesList _output_get))))))
    (Utilities|IsValid _output_get_2
      (:Is%20Valid
        (if (|ChecNullOrObstacle_2 _output_get_2) :!label _label
          _
          (else
            (|LoopCheckNullOrObstacle_2 (Utilities|Array|Get(acopy) (Variables|/Game/Blueprints/grid_BP.grid_BP_C|GetNodesList _output_get) (Math|Random|RandomIntegerinRange 0 (Utilities|Array|Length (Variables|/Game/Blueprints/grid_BP.grid_BP_C|GetNodesList _output_get))))
              (:then
                _)
              (:else
                (goto _label)))))
        (Utilities|IsValid _output_get_2
          (:Is%20Valid
            (Variables|/Script/AntiVirusTactical.GridNode|SetLinkedActor (Variables|Default|GetLinkedNode) _self)
            (Transformation|SetActorLocation _self (Math|Vector|MakeVector (.x (Transformation|GetActorLocation (Variables|Default|GetLinkedNode))) (.y (Transformation|GetActorLocation (Variables|Default|GetLinkedNode))) (+ (.z (Transformation|GetActorLocation (Variables|Default|GetLinkedNode))) 1e+02)) false false)
            (bind _asanti_virus_tactical_game_mode (Utilities|Casting|CastToAntiVirusTacticalGameMode (Game|GetGameMode)))
            (Utilities|IsValid _asanti_virus_tactical_game_mode
              (:Is%20Valid
                (Utilities|Array|Add (Variables|/Script/AntiVirusTactical.AntiVirusTacticalGameMode|GetEnemies _asanti_virus_tactical_game_mode) self)
                (Utilities|IsValid (Variables|Default|GetlifeSystemComponent)
                  (:Is%20Valid
                    _)
                  (:Is%20Not%20Valid
                    (bind _returnvalue_2 (AddComponent|AddLifeSystemComponent self))
                    (bind _output_get_3 (Variables|Default|SetlifeSystemComponent _returnvalue_2))
                    (Utilities|IsValid _output_get_3
                      (:Is%20Valid
                        _))))
                (bind _aslife_widget (Utilities|Casting|CastToLife_Widget (UserInterface|GetUserWidgetObject (Variables|Default|GetLifeWidgetComponent))))
                (Variables|/Game/Widget/Life_Widget.Life_Widget_C|SetOwnerReference _aslife_widget _self_2)
                (Default|LateInit _aslife_widget _self_2)))))))))

(event EventAttack
  (bind _currenttarget (Variables|Default|GetcurrentTarget))
  (Animation|PlayAnimMontage self "/Game/Animations/Weapons/Melee/HitSkill_AMBP.HitSkill_AMBP" 1.0 "default")
  (Utilities|IsValid _currenttarget
    (:Is%20Valid
      (bind _astop_down_character (Utilities|Casting|CastToTopDownCharacter _currenttarget))
      (Class|LifeSystemComponent|RemoveHealth (Variables|/Script/AntiVirusTactical.AntiVirusTacticalCharacter|GetlifeSystemComponent _astop_down_character) (Variables|Default|Getdamage)))))

(event EventSpawnVirus
  (params (_posX :type Integer) (_posY :type Integer))
  (Utilities|IsValid self
    (:Is%20Valid
      (Utilities|IsValid (Variables|Default|GetGrid)
        (:Is%20Valid
          (bind _node (Default|GetLinearIndexwithOffset (Variables|Default|GetGrid) _posX _posY (Variables|Default|GetLinkedNode)))
          (Utilities|IsValid _node
            (:Is%20Valid
              (if (and (not (Variables|/Script/AntiVirusTactical.GridNode|GetisObstacle _node)) (== (Variables|/Script/AntiVirusTactical.GridNode|GetLinkedActor _node) 0))
                (bind _returnvalue (Game|SpawnActorfromClass "VirusCharacter_BP_C" (Math|Transform|MakeTransform (Transformation|GetActorLocation _node)) "Undefined" 0 true 0))
                (Utilities|IsValid _returnvalue
                  (:Is%20Valid
                    (Variables|/Script/AntiVirusTactical.VirusCharacter|SethasPlayed _returnvalue true)
                    (Variables|/Script/AntiVirusTactical.GridNode|SetLinkedActor _node _returnvalue)
                    (Variables|/Script/AntiVirusTactical.VirusCharacter|SetLinkedNode _returnvalue _node)
                    (Variables|VirusCharacter_BP_C|SetGrid _returnvalue (Variables|Default|GetGrid))
                    (Transformation|SetActorLocation _returnvalue (Math|Vector|MakeVector (.x (Transformation|GetActorLocation _node)) (.y (Transformation|GetActorLocation _node)) (+ (.z (Transformation|GetActorLocation _node)) 1e+02)) false false)
                    (bind _asanti_virus_tactical_game_mode (Utilities|Casting|CastToAntiVirusTacticalGameMode (Game|GetGameMode)))
                    (Utilities|Array|Add (Variables|/Script/AntiVirusTactical.AntiVirusTacticalGameMode|GetEnemies _asanti_virus_tactical_game_mode) _returnvalue)
                    (Utilities|IsValid (Variables|/Script/AntiVirusTactical.VirusCharacter|GetlifeSystemComponent _returnvalue)
                      (:Is%20Valid
                        _)
                      (:Is%20Not%20Valid
                        (bind _returnvalue_2 (AddComponent|AddLifeSystemComponent _returnvalue))
                        (bind _output_get (Variables|/Script/AntiVirusTactical.VirusCharacter|SetlifeSystemComponent _returnvalue _returnvalue_2))
                        (Utilities|IsValid _output_get
                          (:Is%20Valid
                            _))))
                    (bind _aslife_widget (Utilities|Casting|CastToLife_Widget (UserInterface|GetUserWidgetObject (Variables|/Script/AntiVirusTactical.VirusCharacter|GetLifeWidgetComponent _returnvalue))))
                    (Variables|/Game/Widget/Life_Widget.Life_Widget_C|SetOwnerReference _aslife_widget _returnvalue)
                    (Default|LateInit _aslife_widget _returnvalue)))))))))))

(event EventRandomMovement
  (params (_randX :type Integer) (_randY :type Integer))
  (bind _grid (Variables|Default|GetGrid))
  (Utilities|IsValid self
    (:Is%20Valid
      (Utilities|IsValid _grid
        (:Is%20Valid
          (bind _node (Default|GetLinearIndexwithOffset _grid _randX _randY (Variables|Default|GetLinkedNode)))
          (Utilities|IsValid _node
            (:Is%20Valid
              (if (and (not (Variables|/Script/AntiVirusTactical.GridNode|GetisObstacle _node)) (== (Variables|/Script/AntiVirusTactical.GridNode|GetLinkedActor _node) 0))
                (Utilities|IsValid (Variables|Default|GetLinkedNode)
                  (:Is%20Valid
                    (Variables|/Script/AntiVirusTactical.GridNode|SetLinkedActor (Variables|Default|GetLinkedNode) 0)
                    (bind _output_get (Variables|Default|SetLinkedNode _node))
                    (Variables|/Script/AntiVirusTactical.GridNode|SetLinkedActor _output_get self)
                    (AI|Navigation|SimpleMovetoLocation (Pawn|GetController) (Transformation|GetActorLocation _output_get))))))))))))

(fn ConstructionScript)

(fn CheckEnemyNearby
  (bind _moverange (Variables|Default|GetmoveRange))
  (bind _returnvalue (- 0 _moverange))
  (Utilities|IsValid (Variables|Default|GetGrid)
    (:Is%20Valid
      (for _index (range _returnvalue _moverange)
        (for _index_2 (range _returnvalue _moverange)
          (bind _node (Default|GetLinearIndexwithOffset (Variables|Default|GetGrid) _index _index_2 (Variables|Default|GetLinkedNode)))
          (Utilities|IsValid _node
            (:Is%20Valid
              (bind _astop_down_character (Utilities|Casting|CastToTopDownCharacter (Variables|/Script/AntiVirusTactical.GridNode|GetLinkedActor _node)))
              (Utilities|Array|Add (LocalVariables|GetActorsNearby) _astop_down_character)))))
      (if (> (Utilities|Array|Length (LocalVariables|GetActorsNearby)) 0)
        (for _array_element (LocalVariables|GetActorsNearby)
          (bind _astop_down_character_2 (Utilities|Casting|CastToTopDownCharacter _array_element))
          (Utilities|IsValid (Variables|/Script/AntiVirusTactical.AntiVirusTacticalCharacter|GetplayerNode _astop_down_character_2)
            (:Is%20Valid
              (bind _returnvalue_2 (Class|NavigationSystemV1|FindPathtoLocationSynchronously (Transformation|GetActorLocation (Variables|Default|GetLinkedNode)) (Transformation|GetActorLocation (Variables|/Script/AntiVirusTactical.AntiVirusTacticalCharacter|GetplayerNode _astop_down_character_2)) 0 0))
              (if (< (Class|NavigationPath|GetPathLength _returnvalue_2) (LocalVariables|GetbestDistance))
                (LocalVariables|SetbestDistance (Class|NavigationPath|GetPathLength _returnvalue_2))
                (LocalVariables|SetNewTarget _array_element)))))
        (bind _output_get (Variables|Default|SetcurrentTarget (LocalVariables|GetNewTarget)))
        (Utilities|IsValid _output_get
          (:Is%20Valid
            (bind _astop_down_character_3 (Utilities|Casting|CastToTopDownCharacter _output_get))
            (for _index_3 (range -1 1)
              (for _index_4 (range -1 1)
                (bind _node_2 (Default|GetLinearIndexwithOffset (Variables|Default|GetGrid) _index_3 _index_4 (Variables|Default|GetLinkedNode)))
                (if (== _node_2 (Variables|/Script/AntiVirusTactical.AntiVirusTacticalCharacter|GetplayerNode _astop_down_character_3))
                  (Variables|Default|SetisOnRangeToAttack true)
                  (return true)
                  (else
                    (Variables|Default|SetisOnRangeToAttack false)))))
            (return true)))
        (else
          (Variables|Default|SetcurrentTarget 0))))
    (:Is%20Not%20Valid
      (return false))))
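; AntiVirusGamemode is a game mode Blueprint that handles the end of a match through win and lose events.
; Each event runs once behind its own DoOnce, clears all widgets and blends the player's view to the level's CameraActor.
; It then shows the matching win or lose screen widget.
; BeginPlay and Tick only call their parent versions.
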(event EventOnWinEvent
  (Utilities|FlowControl|DoOnce false
    (:Completed
      (Viewport|RemoveAllWidgets)
      (bind _returnvalue (Actor|GetActorOfClass "/Script/Engine.CameraActor"))
      (Game|Player|SetViewTargetwithBlend (Game|GetPlayerController 0) _returnvalue 3.0 "VTBlend_Linear" 0.0 false)
      (bind _returnvalue_2 (UserInterface|CreateWidget "/Game/Widget/WinScreen_Widget.WinScreen_Widget_C"))
      (UserInterface|Viewport|AddtoViewport _returnvalue_2 0))))

(event EventOnLoseEvent
  (Utilities|FlowControl|DoOnce false
    (:Completed
      (Viewport|RemoveAllWidgets)
      (bind _returnvalue (Actor|GetActorOfClass "/Script/Engine.CameraActor"))
      (Game|Player|SetViewTargetwithBlend (Game|GetPlayerController 0) _returnvalue 2.0 "VTBlend_Linear" 0.0 false)
      (bind _returnvalue_2 (UserInterface|CreateWidget "/Game/Widget/Lose_Widget.Lose_Widget_C"))
      (UserInterface|Viewport|AddtoViewport _returnvalue_2 0))))

(event EventTick
  (params (DeltaSeconds :type Float%20%28single-precision%29))
  (|CallParentFunction DeltaSeconds))

(event EventBeginPlay
  (|CallParentFunction))

(fn ConstructionScript)